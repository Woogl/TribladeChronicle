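; BP_EnemyAIController is the AI controller for enemy characters, driving them with a behavior tree and perception.
; On possess it runs the behavior tree and stores the pawn's starting location in the InitialLocation blackboard key.
; Perception updates set TargetActor to the sensed actor, or clear it when a stimulus is lost, whichever actor that update concerns.
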(event `self.ReceivePossess`
  (params (PossessedPawn :type "Pawn Object Reference"))
  (`self.RunBehaviorTree` (`self.BTAsset`))
  (`BlackboardComponent.SetValueAsVector` (`AIBlueprintHelperLibrary.GetBlackboard` null) "InitialLocation" (`self.K2_GetActorLocation` PossessedPawn)))

(event `self.AIPerception.OnTargetPerceptionInfoUpdated`
  (params (UpdateInfo :type "ActorPerceptionUpdateInfo Structure (by ref)"))
  (bind (_targetid _target _stimulus) (break `ActorPerceptionUpdateInfo` UpdateInfo))
  (if (`.bSuccessfullySensed` (break `AIStimulus` _stimulus))
    (`BlackboardComponent.SetValueAsObject` (`AIBlueprintHelperLibrary.GetBlackboard` null) "TargetActor" _target)
    (else
      (`BlackboardComponent.ClearValue` (`AIBlueprintHelperLibrary.GetBlackboard` null) "TargetActor"))))

(fn `UserConstructionScript`)