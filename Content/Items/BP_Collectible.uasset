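; BP_Collectible is a pickup that grants a gameplay ability to any overlapping actor that has an Ability System Component.
; On box overlap it gives the configured AbilityClass, then immediately tries to activate it.
; Only if activation succeeds does it also grant GA_EquipWeapon and destroy itself, so a failed activation leaves the pickup in the world.
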(event `self.Box.OnComponentBeginOverlap`
  (params (OverlappedComponent :type "PrimitiveComponent Object Reference") (OtherActor :type "Actor Object Reference") (OtherComp :type "PrimitiveComponent Object Reference") (OtherBodyIndex :type Integer) (bFromSweep :type Boolean) (SweepResult :type "HitResult Structure (by ref)"))
  (bind _returnvalue (`AbilitySystemBlueprintLibrary.GetAbilitySystemComponent` OtherActor))
  (bind _abilityclass (`self.AbilityClass`))
  (if (and (`KismetSystemLibrary.IsValidClass` _abilityclass) (`KismetSystemLibrary.IsValid` _returnvalue))
    (bind _returnvalue_2 (`AbilitySystemComponent.K2_GiveAbility` _returnvalue _abilityclass 0 -1))
    (bind _returnvalue_3 (`AbilitySystemComponent.TryActivateAbility` _returnvalue _returnvalue_2 true))
    (if _returnvalue_3
      (`AbilitySystemComponent.K2_GiveAbility` _returnvalue "/Game/GAS/Abilities/GA_EquipWeapon.GA_EquipWeapon_C" 0 -1)
      (`self.K2_DestroyActor`))))

(fn `UserConstructionScript`)