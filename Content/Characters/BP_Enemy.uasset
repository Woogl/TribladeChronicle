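; Enemy character Blueprint that handles death by switching to a physics ragdoll.
; When health reaches zero, it sends an Event.Death gameplay event to itself, and the health component's death-started callback triggers the ragdoll.
; The mesh simulates physics from the pelvis down, with a velocity impulse carrying and boosting the last movement.
; The first attached sword and shield are each notified through their OnRagdoll functions.
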(event `self.HealthComponent.OnHealthChanged`
  (params (HealthComponent :type "TcHealthComponent Object Reference") (OldValue :type "Float (single-precision)") (NewValue :type "Float (single-precision)") (Instigator :type "Actor Object Reference"))
  (if (<= NewValue 0.0)
    (`AbilitySystemBlueprintLibrary.SendGameplayEventToActor` self (struct :`TagName` "Event.Death"))))

(event `self.HealthComponent.OnDeathStarted`
  (params (OwningActor :type "Actor Object Reference"))
  (`self.EnableRagdoll`))

(event `EnableRagdoll`
  (bind _mesh (`self.Mesh`))
  (bind _returnvalue (`CharacterMovementComponent.GetLastUpdateVelocity` (`self.CharacterMovement`)))
  (`PrimitiveComponent.SetCollisionProfileName` _mesh "Ragdoll" true)
  (`SkeletalMeshComponent.SetAllBodiesBelowSimulatePhysics` _mesh "Pelvis" true true)
  (`PrimitiveComponent.AddImpulse` _mesh (+ _returnvalue (* (`KismetMathLibrary.Normal` _returnvalue) 500.0)) "Pelvis" true)
  (`|ExecutionSequence`
    (:`then_0`
      (for _array_element (`self.GetAttachedActors` true)
        (bind _asbp_sword (cast `/Game/Items/Weapons/BP_Sword` _array_element))
        (`/Game/Items/Weapons/BP_Sword.OnRagdoll` _asbp_sword)
        (break)))
    (:`then_1`
      (for _array_element_2 (`self.GetAttachedActors` true)
        (bind _asbp_shield (cast `/Game/Items/Weapons/BP_Shield` _array_element_2))
        (`/Game/Items/Weapons/BP_Shield.OnRagdoll` _asbp_shield)
        (break)))))

(fn `UserConstructionScript`)