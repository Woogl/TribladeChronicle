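; BP_Hero is the hero character Blueprint, wiring health to the HUD and handling death with a physics ragdoll.
; On BeginPlay it pushes WBP_GameHUD to the game UI layer and caches its health view model.
; Health changes update that view model and send a death gameplay event at zero.
; Death start ragdolls the mesh from the pelvis with a velocity-based impulse, then notifies attached sword and shield actors.
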(event `self.ReceiveBeginPlay`
  (bind (_asynctaskproxy _userwidget) (`AsyncAction_PushContentToLayerForPlayer.PushContentToLayerForPlayer` (`GameplayStatics.GetPlayerController` 0) "/Game/UI/Widgets/WBP_GameHUD.WBP_GameHUD_C" (struct :`TagName` "UI.Layer.Game"))
    (:`AfterPush`
      (bind _aswbp_game_hud (cast `/Game/UI/Widgets/WBP_GameHUD` _userwidget))
      (set `self.VM Health` (`/Game/UI/Widgets/WBP_GameHUD.VM_Health` _aswbp_game_hud)))))

(event `self.HealthComponent.OnHealthChanged`
  (params (HealthComponent :type "TcHealthComponent Object Reference") (OldValue :type "Float (single-precision)") (NewValue :type "Float (single-precision)") (Instigator :type "Actor Object Reference"))
  (`|ExecutionSequence`
    (:`then_0`
      (if (<= NewValue 0.0)
        (`AbilitySystemBlueprintLibrary.SendGameplayEventToActor` self (struct :`TagName` "Event.Death"))))
    (:`then_1`
      (bind _vm_health (`self.VM Health`)
        (:`then`
          (`/Game/UI/ViewModels/VM_Health.SetCurrentHealth` _vm_health NewValue))
        (:`else`)))))

(event `self.HealthComponent.OnDeathStarted`
  (params (OwningActor :type "Actor Object Reference"))
  (`self.EnableRagdoll`))

(event `EnableRagdoll`
  (bind _mesh (`self.Mesh`))
  (bind _returnvalue (`CharacterMovementComponent.GetLastUpdateVelocity` (`self.CharacterMovement`)))
  (`PrimitiveComponent.SetCollisionProfileName` _mesh "TcRagdoll" true)
  (`SkeletalMeshComponent.SetAllBodiesBelowSimulatePhysics` _mesh "Pelvis" true true)
  (`PrimitiveComponent.AddImpulse` _mesh (+ _returnvalue (* (`KismetMathLibrary.Normal` _returnvalue) 500.0)) "Pelvis" true)
  (`|ExecutionSequence`
    (:`then_0`
      (for _array_element (`self.GetAttachedActors` true)
        (bind _asbp_sword (cast `/Game/Items/Weapons/BP_Sword` _array_element))
        (`/Game/Items/Weapons/BP_Sword.OnRagdoll` _asbp_sword)
        (break)))
    (:`then_1`
      (for _array_element_2 (`self.GetAttachedActors` true)
        (bind _asbp_shield (cast `/Game/Items/Weapons/BP_Shield` _array_element_2))
        (`/Game/Items/Weapons/BP_Shield.OnRagdoll` _asbp_shield)
        (break)))))

(fn `UserConstructionScript`)